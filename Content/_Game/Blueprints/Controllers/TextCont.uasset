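; TextCont is a player controller that lets key presses drive a tagged NewBlueprint actor in the level.
; On BeginPlay it finds the first actor tagged "New", casts it to NewBlueprint and stores it as Obj.
; Space Bar calls SetWet on that object and Tab calls SetSet with the controlled pawn.
; Both calls run only with authority, and neither key has a remote branch or RPC in this graph.
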(event EventBeginPlay
  (bind _outactors (Actor|GetAllActorswithTag "New"))
  (bind _asnew_blueprint (Utilities|Casting|CastToNewBlueprint (Utilities|Array|Get(acopy) _outactors)))
  (Variables|Default|SetObj _asnew_blueprint))

(event Input|KeyboardEvents|Tab
  (params (Key :type Key%20Structure :default "None"))
  (:Pressed
    (Networking|SwitchHasAuthority
      (:Authority
        (Default|SetSet (Variables|Default|GetObj) (Pawn|GetControlledPawn))))))

(event Input|KeyboardEvents|SpaceBar
  (params (Key :type Key%20Structure :default "None"))
  (:Pressed
    (Networking|SwitchHasAuthority
      (:Authority
        (Default|SetWet (Variables|Default|GetObj))))))

(fn ConstructionScript)